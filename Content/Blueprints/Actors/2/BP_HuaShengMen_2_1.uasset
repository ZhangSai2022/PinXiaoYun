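; Interactive sectional overhead door (滑升门) actor with labeled parts such as control system, panel, heated window, track, motor and torsion spring.
; On BeginPlay, each part's WBP_JieSao1 widget takes its name from the component's first tag and its description from the 介绍 map.
; Double-clicking the 控制系统3 mesh alternately plays and reverses a timeline that raises and lowers Scene along relative Z.
; Hover and single-click handlers do nothing.
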(event `self.ReceiveBeginPlay`
  (for _array_element (`|MakeArray` (`self.控制系统`) (`self.门板`) (`self.加热视窗`) (`self.轨道`) (`self.电机`) (`self.扭簧`) (`self.塔轮`))
    (`self.set介绍` _array_element)))

(event `set介绍`
  (params (`目标` :type "WidgetComponent Object Reference"))
  (bind _returnvalue (`KismetStringLibrary.Conv_NameToString` (`|GetArrayItem` (`ActorComponent.ComponentTags` `目标`))))
  (bind _aswbp_jie_sao_1 (cast `/Game/Blueprints/UI/Widgets/WBP_JieSao1` (`WidgetComponent.GetWidget` `目标`)))
  (`/Game/Blueprints/UI/Widgets/WBP_JieSao1.set文本` _aswbp_jie_sao_1 (`KismetTextLibrary.Conv_StringToText` _returnvalue) (`KismetTextLibrary.Conv_StringToText` (`BlueprintMapLibrary.Map_Find` (`self.介绍`) _returnvalue))))

(event `self.BP_OnHoverGlowChanged`
  (params (bIsHovered :type Boolean) (SourceComponent :type "StaticMeshComponent Object Reference")))

(event `self.控制系统3.OnClicked`
  (params (TouchedComponent :type "PrimitiveComponent Object Reference") (ButtonPressed :type "Key Structure")))

(event `self.BP_OnStaticMeshDoubleClicked`
  (params (MeshComponent :type "StaticMeshComponent Object Reference"))
  (if (`KismetStringLibrary.EqualEqual_StrStr` (`KismetSystemLibrary.GetObjectName` MeshComponent) "控制系统3")
    (`/Engine/EditorBlueprintResources/StandardMacros.FlipFlop`
      (:`A`
        (bind (_direction `_新建轨道_0`) (`Timeline|时间轴` :!via `PlayFromStart` :!label _label)
          (:`Update`
            (`SceneComponent.K2_SetRelativeLocation` (`self.Scene`) (`KismetMathLibrary.MakeVector` 0.0 0.0 (`KismetMathLibrary.Lerp` 0.0 300.0 `_新建轨道_0`)) false false))))
      (:`B`
        (goto _label :!via `ReverseFromEnd`)))))

(fn `UserConstructionScript`)