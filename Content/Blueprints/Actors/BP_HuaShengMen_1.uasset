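; BP_HuaShengMen_1 is a door actor, apparently a sliding lift door, built from child static mesh actors.
; Its construction script walks all child actors and records each static mesh component with its first material in NewVar.
; An unconnected event graph fragment would swap components tagged "门板" (door panel) to the transparent MI_TouMing material, but it never runs.
; Nothing here reads the cached materials back.
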(fn `UserConstructionScript`
  (for _array_element (`self.GetAllChildActors` true)
    (bind `_as静态网格体actor` (cast `StaticMeshActor` _array_element))
    (bind _staticmeshcomponent (`StaticMeshActor.StaticMeshComponent` `_as静态网格体actor`))
    (`BlueprintMapLibrary.Map_Add` (`self.NewVar`) _staticmeshcomponent (`|GetArrayItem` (`MeshComponent.GetMaterials` _staticmeshcomponent)))))