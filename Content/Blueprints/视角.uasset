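; 视角 (viewpoint) Blueprint provides mouse-driven orbit-style look and zoom controls for a spring-arm setup.
; A flag tracks whether the left mouse button is held, gating mouse axes into controller pitch and yaw input, with yaw inverted.
; The mouse wheel changes the SpringArm length in fixed steps without clamping, with wheel up lengthening it and wheel down shortening it.
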(event `InputAxisKey|MouseY`
  (params (AxisValue :type "Float (single-precision)"))
  (if (`self.鼠标左键点击`)
    (`self.AddControllerPitchInput` AxisValue)))

(event `InputAxisKey|MouseX`
  (params (AxisValue :type "Float (single-precision)"))
  (if (`self.鼠标左键点击`)
    (`self.AddControllerYawInput` (* AxisValue -1.0))))

(event `Key|LeftMouseButton`
  (params (Key :type "Key Structure"))
  (:`Pressed`
    (set `self.鼠标左键点击` true))
  (:`Released`
    (set `self.鼠标左键点击` false)))

(event `self.ReceiveBeginPlay`
  (set `self.鼠标左键点击` false))

(event `Key|MouseScrollUp`
  (params (Key :type "Key Structure"))
  (bind _springarm (`self.SpringArm`))
  (:`Pressed`
    (set `SpringArmComponent.TargetArmLength` (+ (`SpringArmComponent.TargetArmLength` _springarm) 20.0) _springarm)))

(event `Key|MouseScrollDown`
  (params (Key :type "Key Structure"))
  (bind _springarm (`self.SpringArm`))
  (:`Pressed`
    (set `SpringArmComponent.TargetArmLength` (+ (`SpringArmComponent.TargetArmLength` _springarm) -20.0) _springarm)))

(fn `UserConstructionScript`)